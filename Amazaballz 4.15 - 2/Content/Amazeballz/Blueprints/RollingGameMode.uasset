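; RollingGameMode is a game mode for Amazeballz that holds the setup logic for local multiplayer.
; SetPlayers switches on the player count to reset chained DoOnce gates, which are meant to limit how many extra local players get created.
; SetControllerID passes each new player's index to its controlled C_Character.
; BeginPlay is empty and the SetPlayers call in the event graph is disconnected, so this asset never runs the setup itself.
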(event `self.ReceiveBeginPlay`)

(fn `SetControllerID`
  (params (playerController :type "PlayerController Object Reference") (playerID :type Integer))
  (bind _asc_character (cast `C_Character` (`Controller.K2_GetPawn` playerController)))
  (`C_Character.SetIndex` _asc_character playerID))

(fn `SetPlayers`
  (`|ExecutionSequence`
    (:`then_0`
      (switch `/Game/Amazeballz/Blueprints/Enums/E_NumberOfPlayers` (`self.NumberOfPlayersInGame`)
        (:`NewEnumerator2`
          (goto _label :!via `Reset`))
        (:`NewEnumerator3`
          (goto _label_2 :!via `Reset`))
        (:`NewEnumerator4`
          (`|ExecutionSequence`
            (:`then_0`
              (goto _label_2 :!via `Reset`))
            (:`then_1`
              (goto _label_3 :!via `Reset`))))))
    (:`then_1`
      (`/Engine/EditorBlueprintResources/StandardMacros.DoOnce` true :!label _label
        (:`Completed`
          (bind _returnvalue (`GameplayStatics.CreatePlayer` 1 false))
          (`self.SetControllerID` _returnvalue 1)
          (`/Engine/EditorBlueprintResources/StandardMacros.DoOnce` true :!label _label_2
            (:`Completed`
              (bind _returnvalue_2 (`GameplayStatics.CreatePlayer` 2 false))
              (`self.SetControllerID` _returnvalue_2 2)
              (`/Engine/EditorBlueprintResources/StandardMacros.DoOnce` true :!label _label_3
                (:`Completed`
                  (bind _returnvalue_3 (`GameplayStatics.CreatePlayer` 3 false))
                  (`self.SetControllerID` _returnvalue_3 3))))))))))

(fn `UserConstructionScript`)