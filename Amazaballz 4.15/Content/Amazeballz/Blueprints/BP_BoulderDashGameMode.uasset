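; Game mode for the Boulder Dash minigame that sets up a shared camera and decides when the match ends.
; On BeginPlay it points each character's player controller at the first boulder's camera and switches input to game-only.
; Every tick it polls the characters, finishing when none remain or any power component reaches max.
; A DoOnce-guarded finish shows the victory widget, pauses the game and switches to UI-only input.
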(event `self.ReceiveBeginPlay`
  (`self.SetPlayerCamera`)
  (`WidgetBlueprintLibrary.SetInputMode_GameOnly` (`GameplayStatics.GetPlayerController` 0)))

(event `self.ReceiveTick`
  (params (DeltaSeconds :type "Float (single-precision)"))
  (`self.CheckPlayerStatus`))

(fn `CheckPlayerStatus`
  (bind _outactors (`GameplayStatics.GetAllActorsOfClass` "/Script/Amazaballz.C_Character"))
  (`|ExecutionSequence`
    (:`then_0`
      ;[1 1 1] If all players have died
      (if (== (`KismetArrayLibrary.Array_Length` _outactors) 0)
        ;[1 1 1] The Game has finished.
        (`self.GameFinished` :!label _label)))
    (:`then_1`
      ;[1 1 1] Checking power levels from the players.
      (for _array_element _outactors
        (bind _returnvalue (`self.GetComponentByClass` _array_element "/Script/Amazaballz.C_PowerComponent"))
        (`/Engine/EditorBlueprintResources/StandardMacros.IsValid` _returnvalue
          (:`Is Valid`
            (bind _returnvalue_2 (`C_PowerComponent.IsAtMax` _returnvalue))
            (if _returnvalue_2
              (goto _label)))
          (:`Is Not Valid`
            (`KismetSystemLibrary.PrintString` "INVALID POWER COMPONENT")))))))

(fn `GameFinished`
  (locals (victory_widget_ :type "/Game/Amazeballz/Blueprints/Widgets/BP_VictoryBoulderDash Object Reference"))
  (bind _returnvalue (`GameplayStatics.GetPlayerController` 0))
  (`/Engine/EditorBlueprintResources/StandardMacros.DoOnce` false
    (:`Completed`
      (bind _returnvalue_2 (`|CreateWidget` "/Game/Amazeballz/Blueprints/Widgets/BP_VictoryBoulderDash.BP_VictoryBoulderDash_C"))
      (bind _output_get (set `local.victory_widget_` _returnvalue_2))
      (`UserWidget.AddToViewport` _output_get 0)
      (set `PlayerController.bShowMouseCursor` true _returnvalue)
      (`GameplayStatics.SetGamePaused` true)
      (`WidgetBlueprintLibrary.SetInputMode_UIOnlyEx` _returnvalue))))

(fn `SetPlayerCamera`
  (set `self.bFindCameraComponentWhenViewTarget` true)
  (bind _outactors (`GameplayStatics.GetAllActorsOfClass` "/Script/Amazaballz.C_Character"))
  (for _array_element _outactors
    (bind _returnvalue (`C_Character.GetIndex` _array_element))
    (bind _outactors_2 (`GameplayStatics.GetAllActorsOfClass` "/Game/Amazeballz/Blueprints/Objects/BP_Boulder.BP_Boulder_C"))
    (`PlayerController.SetViewTargetWithBlend` (`GameplayStatics.GetPlayerController` _returnvalue) (`KismetArrayLibrary.Array_Get` _outactors_2) 0.0 "VTBlend_Linear" 0.0 false)))

(fn `UserConstructionScript`
  (`parent.UserConstructionScript`))