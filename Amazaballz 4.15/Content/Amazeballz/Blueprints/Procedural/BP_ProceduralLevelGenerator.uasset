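; Procedural level generator that builds a grid map from random streaming level chunks when play begins.
; It clears old chunks, then loops the map size, instancing a random named streaming level per cell.
; Each instance is placed by chunk size around a centred origin, optionally with random quarter-turn yaw, then set loaded and visible.
; A fixed starting-chunk path exists but is disconnected and noted as broken.
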(event `self.ReceiveBeginPlay`
  (`self.ProcedurallyGenerate`))

(fn `Add Chunk`
  (params (x_index :type Integer) (y_index :type Integer) (chunk_names :type "Array of Name") (random_rotation :type Boolean) (select_random_chunk :type Boolean))
  (if select_random_chunk
    ;[0 0.3265 1] Random Chunk Generation
    (bind _returnvalue (`LevelStreaming.CreateInstance` (`GameplayStatics.GetStreamingLevel` (`KismetArrayLibrary.Array_Get` chunk_names (`KismetMathLibrary.RandomInteger` (`KismetArrayLibrary.Array_Length` chunk_names)))) (`KismetStringLibrary.Concat_StrStr` (`KismetStringLibrary.Conv_IntToString` x_index) "x" (`KismetStringLibrary.Conv_IntToString` y_index))))
    (`self.CreateLevelChunk` _returnvalue x_index y_index random_rotation)
    (else
      ;[0 0.3265 1] Standard Chunk Generation
      (for (_array_element _array_index) chunk_names
        (bind _returnvalue_2 (`LevelStreaming.CreateInstance` (`GameplayStatics.GetStreamingLevel` _array_element) (`KismetStringLibrary.Concat_StrStr` (`KismetStringLibrary.Conv_IntToString` x_index) "x" (`KismetStringLibrary.Conv_IntToString` y_index))))
        (`self.CreateLevelChunk` _returnvalue_2 _array_index y_index random_rotation)
        (`KismetSystemLibrary.PrintString` "Added new Chunk")))))

(fn `ClearLevelChunks`
  (`self.ClearChunks`))

(fn `CreateLevelChunk`
  (params (level :type "LevelStreaming Object Reference") (x_index :type Integer) (y_index :type Integer) (random_rotation :type Boolean))
  (bind _chunk_size_x_ (`self.chunk_size_x_`))
  (bind _chunk_size_y_ (`self.chunk_size_y_`))
  (bind _returnvalue (- (* x_index _chunk_size_x_) (* (* (`self.map_size_x_`) _chunk_size_x_) 0.5)))
  (bind _returnvalue_2 (- (* y_index _chunk_size_y_) (* (* (`self.map_size_y_`) _chunk_size_y_) 0.5)))
  ;[1 1 1] Creating the level based on map size and chunk size.
  (if random_rotation
    (set `LevelStreaming.LevelTransform` (`KismetMathLibrary.MakeTransform` (`KismetMathLibrary.MakeVector` _returnvalue _returnvalue_2) (`KismetMathLibrary.MakeRotator` 0.0 0.0 (* (`KismetMathLibrary.RandomInteger` 4) 90.0))) level)
    (else
      (set `LevelStreaming.LevelTransform` (`KismetMathLibrary.MakeTransform` (`KismetMathLibrary.MakeVector` _returnvalue _returnvalue_2) (`KismetMathLibrary.MakeRotator` 0.0)) level)))
  (set `LevelStreaming.bShouldBeLoaded` true level)
  (set `LevelStreaming.bShouldBeVisible` true level)
  (`self.AddChunkForClass` level))

(fn `ProcedurallyGenerate`
  (`self.ClearLevelChunks`)
  ;[1 1 1] Creates the random level building up the chunks.
  (for _index (range (+ (`self.map_size_x_`) 1))
    (for _index_2 (range (+ (`self.map_size_y_`) 1))
      (`self.Add Chunk` _index _index_2 (`self.chunk_names_`) true true))))

(fn `SetStartingChunks`
  (bind _starting_chunks_ (`self.starting_chunks_`))
  (if (> (`KismetArrayLibrary.Array_Length` _starting_chunks_) 0)
    (`self.Add Chunk` 0 0 _starting_chunks_)))

(fn `UserConstructionScript`)