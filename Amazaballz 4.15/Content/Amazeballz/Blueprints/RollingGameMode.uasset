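; RollingGameMode is the game mode for Amazeballz that spawns local players for a multiplayer match at BeginPlay.
; SetPlayers always creates a second player, and adds a third or fourth according to NumberOfPlayersInGame.
; The player count resets chained DoOnce nodes that act as gates on the extra CreatePlayer calls.
; SetControllerID passes each new player's ID to its BP_Player pawn through SetIndex.
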(event `self.ReceiveBeginPlay`
  (`self.SetPlayers`))

(fn `SetControllerID`
  (params (playerController :type "PlayerController Object Reference") (playerID :type Integer))
  (bind _asbp_player (cast `/Game/Amazeballz/Blueprints/Characters/BP_Player` (`Controller.K2_GetPawn` playerController)))
  (`C_Player.SetIndex` _asbp_player playerID))

(fn `SetPlayers`
  (`|ExecutionSequence`
    (:`then_0`
      (switch `/Game/Amazeballz/Blueprints/Enums/E_NumberOfPlayers` (`self.NumberOfPlayersInGame`)
        (:`NewEnumerator3`
          (goto _label :!via `Reset`))
        (:`NewEnumerator4`
          (`|ExecutionSequence`
            (:`then_0`
              (goto _label :!via `Reset`))
            (:`then_1`
              (goto _label_2 :!via `Reset`))))))
    (:`then_1`
      (bind _returnvalue (`GameplayStatics.CreatePlayer` 1))
      (`self.SetControllerID` _returnvalue 1)
      (`/Engine/EditorBlueprintResources/StandardMacros.DoOnce` true :!label _label
        (:`Completed`
          (bind _returnvalue_2 (`GameplayStatics.CreatePlayer` 2))
          (`self.SetControllerID` _returnvalue_2 2)
          (`/Engine/EditorBlueprintResources/StandardMacros.DoOnce` true :!label _label_2
            (:`Completed`
              (bind _returnvalue_3 (`GameplayStatics.CreatePlayer` 3))
              (`self.SetControllerID` _returnvalue_3 3))))))))

(fn `UserConstructionScript`)